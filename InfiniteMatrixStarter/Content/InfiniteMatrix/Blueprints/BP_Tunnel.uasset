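; BP_Tunnel is a tunnel segment with a rotating holed wall, plus an optional health package and enemy.
; Its exit trigger has TunnelSpawner spawn another tunnel and destroys this one, adding score and round only without a wall collision.
; Overlaps update BP_Player health, score and death, shake the camera on hits, and consume bullets.
; Uncalled-here helper functions randomize the wall mesh and roll, and keep or remove each pickup and enemy.
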(event OnComponentBeginOverlap(TriggrtZone)
  (params (OverlappedComponent :type Primitive%20Component%20Object%20Reference) (OtherActor :type Actor%20Object%20Reference) (OtherComp :type Primitive%20Component%20Object%20Reference) (OtherBodyIndex :type Integer) (bFromSweep :type Boolean) (SweepResult :type Hit%20Result%20Structure%20%28by%20ref%29))
  (bind _asbp_player (Utilities|Casting|CastToBP_Player OtherActor))
  (if (Variables|Default|GetCollision%20with%20Wall)
    (Default|SpawnTunnelatSpawnPoint (Variables|Default|GetTunnelSpawner))
    (Actor|DestroyActor)
    (else
      (bind _output_get (Variables|/Game/InfiniteMatrix/Blueprints/BP_Player.BP_Player_C|SetScoreVolume _asbp_player (+ (Variables|/Game/InfiniteMatrix/Blueprints/BP_Player.BP_Player_C|GetScoreVolume _asbp_player) 1)))
      (Default|UpdateScoreVolume (Variables|/Game/InfiniteMatrix/Blueprints/BP_Player.BP_Player_C|GetScore%20Number _asbp_player) _output_get)
      (Variables|/Game/InfiniteMatrix/Blueprints/BP_Player.BP_Player_C|Setround _asbp_player (+ (Variables|/Game/InfiniteMatrix/Blueprints/BP_Player.BP_Player_C|Getround _asbp_player) 1))
      (Default|SpawnTunnelatSpawnPoint (Variables|Default|GetTunnelSpawner))
      (Actor|DestroyActor))))

(event OnComponentBeginOverlap(Enemy)
  (params (OverlappedComponent :type Primitive%20Component%20Object%20Reference) (OtherActor :type Actor%20Object%20Reference) (OtherComp :type Primitive%20Component%20Object%20Reference) (OtherBodyIndex :type Integer) (bFromSweep :type Boolean) (SweepResult :type Hit%20Result%20Structure%20%28by%20ref%29))
  (bind _asbp_bullet (Utilities|Casting|CastToBP_Bullet OtherActor)
    (:then
      (Actor|DestroyActor _asbp_bullet)
      (Components|DestroyComponent (Variables|Default|GetEnemy))
      (bind _asbp_player (Utilities|Casting|CastToBP_Player (Game|Player|GetPlayerPawn 0)))
      (bind _output_get (Variables|/Game/InfiniteMatrix/Blueprints/BP_Player.BP_Player_C|SetScoreVolume _asbp_player (+ (Variables|/Game/InfiniteMatrix/Blueprints/BP_Player.BP_Player_C|GetScoreVolume _asbp_player) 1)))
      (Default|UpdateScoreVolume (Variables|/Game/InfiniteMatrix/Blueprints/BP_Player.BP_Player_C|GetScore%20Number _asbp_player) _output_get))
    (:CastFailed
      (bind _asbp_player_2 (Utilities|Casting|CastToBP_Player OtherActor))
      (Camera|PlayWorldCameraShake "/Game/InfiniteMatrix/Blueprints/BP_Shake.BP_Shake_C" (Transformation|GetWorldLocation (Variables|/Game/InfiniteMatrix/Blueprints/BP_Player.BP_Player_C|GetCamera _asbp_player_2)) 0.0 5e+02)
      (Components|DestroyComponent (Variables|Default|GetEnemy))
      (bind _output_get_2 (Variables|/Game/InfiniteMatrix/Blueprints/BP_Player.BP_Player_C|SetHealthVolume _asbp_player_2 (- (Variables|/Game/InfiniteMatrix/Blueprints/BP_Player.BP_Player_C|GetHealthVolume _asbp_player_2) 5.0)))
      (Default|UpdateHealthBar (Variables|/Game/InfiniteMatrix/Blueprints/BP_Player.BP_Player_C|GetHealthBar _asbp_player_2) _output_get_2)
      (if (<= _output_get_2 0.0)
        (Variables|/Game/InfiniteMatrix/Blueprints/BP_Player.BP_Player_C|SetisDead _asbp_player_2 true)
        (Default|DisplayRestart _asbp_player_2)))))

(event OnComponentBeginOverlap(WallMesh)
  (params (OverlappedComponent :type Primitive%20Component%20Object%20Reference) (OtherActor :type Actor%20Object%20Reference) (OtherComp :type Primitive%20Component%20Object%20Reference) (OtherBodyIndex :type Integer) (bFromSweep :type Boolean) (SweepResult :type Hit%20Result%20Structure%20%28by%20ref%29))
  (bind _asbp_player (Utilities|Casting|CastToBP_Player OtherActor)
    (:then
      (Camera|PlayWorldCameraShake "/Game/InfiniteMatrix/Blueprints/BP_Shake.BP_Shake_C" (Transformation|GetWorldLocation (Variables|/Game/InfiniteMatrix/Blueprints/BP_Player.BP_Player_C|GetCamera _asbp_player)) 0.0 5e+02)
      (Variables|Default|SetCollision%20with%20Wall true)
      (bind _output_get (Variables|/Game/InfiniteMatrix/Blueprints/BP_Player.BP_Player_C|SetHealthVolume _asbp_player (- (Variables|/Game/InfiniteMatrix/Blueprints/BP_Player.BP_Player_C|GetHealthVolume _asbp_player) 1e+01)))
      (Default|UpdateHealthBar (Variables|/Game/InfiniteMatrix/Blueprints/BP_Player.BP_Player_C|GetHealthBar _asbp_player) _output_get)
      (if (<= _output_get 0.0)
        (Variables|/Game/InfiniteMatrix/Blueprints/BP_Player.BP_Player_C|SetisDead _asbp_player true)
        (Default|DisplayRestart _asbp_player)))
    (:CastFailed
      (bind _asbp_bullet (Utilities|Casting|CastToBP_Bullet OtherActor))
      (Actor|DestroyActor _asbp_bullet))))

(event OnComponentBeginOverlap(HealthPackage)
  (params (OverlappedComponent :type Primitive%20Component%20Object%20Reference) (OtherActor :type Actor%20Object%20Reference) (OtherComp :type Primitive%20Component%20Object%20Reference) (OtherBodyIndex :type Integer) (bFromSweep :type Boolean) (SweepResult :type Hit%20Result%20Structure%20%28by%20ref%29))
  (bind _healthpackage (Variables|Default|GetHealthPackage))
  (bind _asbp_player (Utilities|Casting|CastToBP_Player OtherActor)
    (:then
      (if (> (+ (Variables|/Game/InfiniteMatrix/Blueprints/BP_Player.BP_Player_C|GetHealthVolume _asbp_player) 2e+01) 1e+02)
        (bind _output_get (Variables|/Game/InfiniteMatrix/Blueprints/BP_Player.BP_Player_C|SetHealthVolume _asbp_player 1e+02))
        (Default|UpdateHealthBar (Variables|/Game/InfiniteMatrix/Blueprints/BP_Player.BP_Player_C|GetHealthBar _asbp_player) _output_get)
        (Components|DestroyComponent _healthpackage)
        (else
          (bind _output_get_2 (Variables|/Game/InfiniteMatrix/Blueprints/BP_Player.BP_Player_C|SetHealthVolume _asbp_player (+ (Variables|/Game/InfiniteMatrix/Blueprints/BP_Player.BP_Player_C|GetHealthVolume _asbp_player) 2e+01)))
          (Default|UpdateHealthBar (Variables|/Game/InfiniteMatrix/Blueprints/BP_Player.BP_Player_C|GetHealthBar _asbp_player) _output_get_2)
          (Components|DestroyComponent _healthpackage))))
    (:CastFailed
      (bind _asbp_bullet (Utilities|Casting|CastToBP_Bullet OtherActor))
      (Actor|DestroyActor _asbp_bullet)
      (Components|DestroyComponent (Variables|Default|GetHealthPackage)))))

(event EventBeginPlay)

(event EventTick
  (params (DeltaSeconds :type Float%20%28single-precision%29))
  (Transformation|AddLocalRotation (Variables|Default|GetWallMesh) (Math|Rotator|MakeRotator (* DeltaSeconds (Variables|Default|GetRotateSpeed)) 0.0 0.0) false false))

(fn ConstructionScript)

(fn RandomizeWall
  (Components|StaticMesh|SetStaticMesh (Variables|Default|GetWallMesh) (Utilities|Select :Index (Math|Random|RandomIntegerinRange 0 3) :Option%200 "/Game/InfiniteMatrix/Meshes/SM_Hole_01.SM_Hole_01" :Option%201 "/Game/InfiniteMatrix/Meshes/SM_Hole_02.SM_Hole_02" :Option%202 "/Game/InfiniteMatrix/Meshes/SM_Hole_03.SM_Hole_03" :Option%203 "/Game/InfiniteMatrix/Meshes/SM_Hole_04.SM_Hole_04"))
  (Transformation|AddLocalRotation (Variables|Default|GetWallMesh) (Math|Rotator|MakeRotator (Math|Random|RandomFloatinRange 0.0 3.6e+02) 0.0 0.0) false false))

(fn HasHealthPackage
  (bind _healthpackage (Variables|Default|GetHealthPackage))
  (if (>= (Math|Random|RandomIntegerinRange 0 8) 1)
    (Components|DestroyComponent _healthpackage)
    (else
      (Transformation|SetRelativeLocation _healthpackage (Math|Vector|MakeVector (Math|Random|RandomFloatinRange 7e+02 2.5e+03) (Math|Random|RandomFloatinRange -15.0 5.9e+02) (Math|Random|RandomFloatinRange -627.0 -1.09e+03)) false false))))

(fn HasEnemy
  (bind _enemy (Variables|Default|GetEnemy))
  (if (>= (Math|Random|RandomIntegerinRange 0 8) 1)
    (Components|DestroyComponent _enemy)
    (else
      (Transformation|SetRelativeLocation _enemy (Math|Vector|MakeVector (Math|Random|RandomFloatinRange 1e+03 2.5e+03) (Math|Random|RandomFloatinRange -3.2e+02 3.2e+02) (Math|Random|RandomFloatinRange -2.5e+02 2.5e+02)) false false))))